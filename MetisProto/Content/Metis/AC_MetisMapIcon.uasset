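; Actor component that gives its owning actor a map icon, built as a flat-scaled static mesh placed high above it.
; On BeginPlay it adds the mesh to the owner, applies the configured scale and material, and disables shadows, collision and visibility to the owner.
; UpdateIconRotation sets the icon's world rotation, leaving its relative and additive flags unused.
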(event EventBeginPlay
  (bind _iconscale (Variables|Default|GetIconScale))
  (bind _returnvalue (Game|AddComponentbyClass (Components|GetOwner) "/Script/Engine.StaticMeshComponent" false))
  (bind _output_get (Variables|Default|SetIconMesh _returnvalue))
  (Components|StaticMesh|SetStaticMesh _output_get "/Game/Metis/SM_MetisMapIcon.SM_MetisMapIcon")
  (Transformation|SetRelativeLocationAndRotation _output_get "0.000000,0.000000,999.000000" "0, 0, 0" false false)
  (Transformation|SetRelativeScale3D _output_get (Math|Vector|MakeVector _iconscale _iconscale 1.0))
  (Rendering|Material|SetMaterial _output_get 0 (Variables|Default|GetIconMaterial))
  (Rendering|SetCastShadow _output_get false)
  (Class|PrimitiveComponent|SetOwnerNoSee _output_get true)
  (Collision|SetCollisionEnabled _output_get "NoCollision"))

(event EventTick
  (params (DeltaSeconds :type Float%20%28single-precision%29)))

(fn UpdateIconRotation
  (params (NewRotation :type Rotator) (IsRelative :type Boolean) (IsAdditive :type Boolean))
  (Transformation|SetWorldRotation (Variables|Default|GetIconMesh) NewRotation false false))