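; BP_MetisLocation is a location marker actor that carries a Metis map icon and a trigger sphere.
; The icon starts at a 90-degree yaw, then each Tick matches the player pawn's yaw plus that offset while the pawn's AC_MetisMapTarget is following the player.
; Overlapping the sphere with a Player-tagged actor only prints a "Location Visited" message.
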(event OnComponentBeginOverlap(Sphere)
  (params (OverlappedComponent :type Primitive%20Component%20Object%20Reference) (OtherActor :type Actor%20Object%20Reference) (OtherComp :type Primitive%20Component%20Object%20Reference) (OtherBodyIndex :type Integer) (bFromSweep :type Boolean) (SweepResult :type Hit%20Result%20Structure%20%28by%20ref%29))
  (if (Actor|ActorHasTag OtherActor "Player")
    (Development|PrintString "Location Visited")))

(event EventBeginPlay
  (Default|UpdateIconRotation (Variables|Default|GetAC_MetisMapIcon) "0.000000,90.000000,0.000000" false false))

(event EventTick
  (params (DeltaSeconds :type Float%20%28single-precision%29))
  (bind _returnvalue (Game|Player|GetPlayerPawn 0))
  (if (Variables|/Game/Metis/AC_MetisMapTarget.AC_MetisMapTarget_C|GetIsFollowingPlayer (Actor|GetComponentbyClass _returnvalue "/Game/Metis/AC_MetisMapTarget.AC_MetisMapTarget_C"))
    (Default|UpdateIconRotation (Variables|Default|GetAC_MetisMapIcon) (Math|Rotator|MakeRotator 0.0 0.0 (+ 9e+01 (.yaw (Transformation|GetActorRotation _returnvalue)))) false false)))

(fn ConstructionScript)