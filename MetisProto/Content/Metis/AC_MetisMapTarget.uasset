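; Actor component for the Metis minimap that, when flagged as the player, sets up the minimap at BeginPlay.
; It creates and displays the minimap widget, then adds an orthographic scene capture above the owner that writes to the minimap render target.
; Setup requires the owner to have the "Player" tag, otherwise it prints a warning.
; Targets not flagged as player do nothing here.
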(event EventBeginPlay
  (bind _returnvalue (Components|GetOwner))
  (if (Variables|Default|GetIsPlayer)
    (if (Actor|ActorHasTag _returnvalue "Player")
      (bind _returnvalue_2 (UserInterface|CreateWidget "/Game/Metis/WB_MetisMinimap.WB_MetisMinimap_C" (Game|GetPlayerController 0)))
      (UserInterface|Viewport|AddtoViewport _returnvalue_2 0)
      (bind _returnvalue_3 (Game|AddComponentbyClass (Components|GetOwner) "/Script/Engine.SceneCaptureComponent2D" false (Math|Transform|MakeTransform "0.000000,0.000000,300.000000" "-90.000000,0.000000,0.000000" "1.000000,1.000000,1.000000")))
      (Variables|/Script/Engine.SceneCaptureComponent2D|SetTextureTarget _returnvalue_3 "/Game/Metis/RT_MetisMinimap.RT_MetisMinimap")
      (Variables|/Script/Engine.SceneCaptureComponent2D|SetProjectionType _returnvalue_3 "Orthographic")
      (Variables|/Script/Engine.SceneCaptureComponent2D|SetOrthoWidth _returnvalue_3 2e+03)
      (else
        (Development|PrintText (Utilities|Text|FormatText "Non-Player Actor {Actor Name} tried to use Metis as player! 
Make sure your player actor has \"Player\" tag." _returnvalue))))))